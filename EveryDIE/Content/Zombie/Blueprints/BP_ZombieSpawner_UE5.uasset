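; Zombie spawner actor that spawns a configurable zombie type, passing in material, sounds, health and attack damage.
; Spawn loops over the count, placing zombies at random reachable points in a radius with randomized yaw and scale, retrying after failed lookups.
; Spawn_2 and SpawnZombie spawn one at the spawner, decrementing the count; SpawnZombie also randomizes transform and sets QuickChase.
; Two guarded functions start looping SpawnZombie timers, still limited by the count.
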(event `Spawn`
  (bind _returnvalue (`KismetMathLibrary.RandomFloatInRange` 0.9 1.1))
  (bind (_randomlocation _returnvalue_2) (`NavigationSystemV1.K2_GetRandomReachablePointInRadius` (`self.K2_GetActorLocation`) (`self.SpawnRadius`) null null))
  (for _ (range (`self.NumberOfZombies`))
    (if _returnvalue_2 :!label _label
      (`|SpawnActorFromClass` (`self.ZombieType`) (`KismetMathLibrary.MakeTransform` _randomlocation (`KismetMathLibrary.MakeRotator` 0.0 0.0 (`KismetMathLibrary.RandomFloatInRange` 0.0 360.0)) (`KismetMathLibrary.MakeVector` _returnvalue _returnvalue _returnvalue)) "AdjustIfPossibleButAlwaysSpawn" "MultiplyWithRoot" null (`self.Material`) (`self.Ambient Sound`) (`self.Roar Sound`) (`self.Death Sound`) (`self.Health`) (`self.Attack Damage`) null)
      (else
        (`KismetSystemLibrary.Delay` 0.1)
        (goto _label)))))

(event `Spawn_2`
  (bind _numberofzombies (`self.NumberOfZombies`))
  (if (> _numberofzombies 0)
    (set `self.NumberOfZombies` (- _numberofzombies 1))
    (`|SpawnActorFromClass` (`self.ZombieType`) (`KismetMathLibrary.MakeTransform` (`self.K2_GetActorLocation`)) "AdjustIfPossibleButAlwaysSpawn" "MultiplyWithRoot" null (`self.Material`) (`self.Ambient Sound`) (`self.Roar Sound`) (`self.Death Sound`) (`self.Health`) (`self.Attack Damage`) null)
    (else
      (`KismetSystemLibrary.PrintString` "empty"))))

(fn `Spawn_by_TImer_10`
  (if (not (`self.infinite spawn2`))
    (set `self.infinite spawn2` true)
    (`KismetSystemLibrary.K2_SetTimer` null "SpawnZombie" 10.0 true false -10.0)))

(fn `Spawn_by_Timer_15`
  (if (not (`self.infinite spawn`))
    (set `self.infinite spawn` true)
    (`KismetSystemLibrary.K2_SetTimer` null "SpawnZombie" 15.0 true false -15.0)))

(fn `SpawnZombie`
  (bind _returnvalue (`KismetMathLibrary.RandomFloatInRange` 0.9 1.1))
  (bind _numberofzombies (`self.NumberOfZombies`))
  (if (> _numberofzombies 0)
    (set `self.NumberOfZombies` (- _numberofzombies 1))
    (bind _returnvalue_2 (`|SpawnActorFromClass` (`self.ZombieType`) (`KismetMathLibrary.MakeTransform` (`self.K2_GetActorLocation`) (`KismetMathLibrary.MakeRotator` 0.0 0.0 (`KismetMathLibrary.RandomFloatInRange` 0.0 360.0)) (`KismetMathLibrary.MakeVector` _returnvalue _returnvalue _returnvalue)) "AdjustIfPossibleButAlwaysSpawn" "MultiplyWithRoot" null (`self.Material`) (`self.Ambient Sound`) (`self.Roar Sound`) (`self.Death Sound`) (`self.Health`) (`self.Attack Damage`) null))
    (set `/Game/Zombie/Blueprints/BP_Zombie_Pawn_UE5.Quick_Chase` (`self.Quick_Chasing`) _returnvalue_2)
    (else
      (`KismetSystemLibrary.PrintString` "empty"))))

(fn `UserConstructionScript`)