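; Player inventory component that handles item pickup, loot boxes and toggling the WB_Inventory widget.
; Interact runs a sphere trace around the player: Ammo feeds the gun magazine, while other items stack or fill empty slots.
; Shoes, flashlight and vest pickups also set character flags or speed.
; Boxes become random items through chained re-rolls, with a separate valuable-box table; the normal box's flashlight branch never reaches the spawn.
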(event Custom|Inventory
  (bind _returnvalue (Game|GetPlayerController 0))
  (bind _inventorywidget (Variables|Default|GetInventorywidget))
  (if (Widget|IsVisible (Variables|Default|GetInventorywidget))
    (Widget|RemovefromParent _inventorywidget)
    (Variables|/Script/Engine.PlayerController|SetbShowMouseCursor _returnvalue false)
    (Input|SetInputModeGameOnly _returnvalue false)
    (else
      (Variables|/Script/Engine.PlayerController|SetbShowMouseCursor _returnvalue true)
      (Input|SetInputModeGameandUI _returnvalue 0 "DoNotLock" true false)
      (UserInterface|Viewport|AddtoViewport _inventorywidget 0))))

(event Custom|interaction
  (bind _returnvalue (Game|GetPlayerCharacter 0))
  (bind _returnvalue_2 (Transformation|GetActorLocation _returnvalue))
  (bind _returnvalue_3 (+ _returnvalue_2 "0.000000,0.000000,-50.000000"))
  (bind _outhit (Collision|SphereTraceByChannel _returnvalue_3 _returnvalue_3 2e+02 "TraceTypeQuery1" false (Variables|Default|GetFloor) "None"))
  (bind _asbp_item (Utilities|Casting|CastToBP_Item (.HitActor (Collision|BreakHitResult _outhit)))
    (:then
      (if (Utilities|Enum|Equal(Enum) (.Name (Utilities|Struct|BreakS_ItemStruct (Variables|/Game/Inventory/Blueprints/BP_Item.BP_Item_C|GetItem _asbp_item))) (Variables|Default|GetAmmo))
        (bind _asbp_crosshair_character (Utilities|Casting|CastToBP_CrosshairCharacter (Game|Player|GetPlayerPawn 0)))
        (bind _asbp_weap_gun (Utilities|Casting|CastToBP_Weap_Gun (Variables|/Game/CT_Components/Demos/Demo_CrosshairSystem/ThirdPerson/BP_CrosshairCharacter.BP_CrosshairCharacter_C|GetWeapon _asbp_crosshair_character)))
        (Variables|/Game/CT_Components/Demos/Demo_CrosshairSystem/ThirdPerson/Weaps/BP_Weap_Gun.BP_Weap_Gun_C|Setmagazine _asbp_weap_gun (+ (Variables|/Game/CT_Components/Demos/Demo_CrosshairSystem/ThirdPerson/Weaps/BP_Weap_Gun.BP_Weap_Gun_C|Getmagazine _asbp_weap_gun) (.Quantity (Utilities|Struct|BreakS_ItemStruct (Variables|/Game/Inventory/Blueprints/BP_Item.BP_Item_C|GetItem _asbp_item)))))
        (Actor|DestroyActor _asbp_item)
        (else
          (for (_array_element _array_index) (Variables|Default|GetItems)
            (Utilities|IsValid _asbp_item
              (:Is%20Valid
                (if (Math|Boolean|ANDBoolean (Utilities|Enum|Equal(Enum) (.Name (Utilities|Struct|BreakS_ItemStruct _array_element)) (.Name (Utilities|Struct|BreakS_ItemStruct (Variables|/Game/Inventory/Blueprints/BP_Item.BP_Item_C|GetItem _asbp_item)))) (.Stackable (Utilities|Struct|BreakS_ItemStruct (Variables|/Game/Inventory/Blueprints/BP_Item.BP_Item_C|GetItem _asbp_item))) (<= (+ (.Quantity (Utilities|Struct|BreakS_ItemStruct _array_element)) (.Quantity (Utilities|Struct|BreakS_ItemStruct (Variables|/Game/Inventory/Blueprints/BP_Item.BP_Item_C|GetItem _asbp_item)))) 5))
                  (Utilities|Array|SetArrayElem (Variables|Default|GetItems) _array_index (Utilities|Struct|MakeS_ItemStruct (.name (Variables|/Game/Inventory/Blueprints/BP_Item.BP_Item_C|GetItem _asbp_item)) (.stackable (Variables|/Game/Inventory/Blueprints/BP_Item.BP_Item_C|GetItem _asbp_item)) (+ (.Quantity (Utilities|Struct|BreakS_ItemStruct _array_element)) (.Quantity (Utilities|Struct|BreakS_ItemStruct (Variables|/Game/Inventory/Blueprints/BP_Item.BP_Item_C|GetItem _asbp_item)))) (.mesh (Variables|/Game/Inventory/Blueprints/BP_Item.BP_Item_C|GetItem _asbp_item)) (.thumnail (Variables|/Game/Inventory/Blueprints/BP_Item.BP_Item_C|GetItem _asbp_item))))
                  (Default|LoadInventory (Variables|Default|GetInventorywidget) self :!label _label)
                  (if (Utilities|Enum|Equal(Enum) (.Name (Utilities|Struct|BreakS_ItemStruct (Variables|/Game/Inventory/Blueprints/BP_Item.BP_Item_C|GetItem _asbp_item))) (Variables|Default|GetShoes))
                    (CallFunction|ShoesGetSpeedChange)
                    (elif (Utilities|Enum|Equal(Enum) (.Name (Utilities|Struct|BreakS_ItemStruct (Variables|/Game/Inventory/Blueprints/BP_Item.BP_Item_C|GetItem _asbp_item))) (Variables|Default|GetFlashLight))
                      (CallFunction|FlashlightGet)
                      (elif (Utilities|Enum|Equal(Enum) (.Name (Utilities|Struct|BreakS_ItemStruct (Variables|/Game/Inventory/Blueprints/BP_Item.BP_Item_C|GetItem _asbp_item))) (Variables|Default|GetVest))
                        (CallFunction|VestGet))))
                  (Actor|DestroyActor _asbp_item)
                  (elif (== (.Quantity (Utilities|Struct|BreakS_ItemStruct _array_element)) 0)
                    (Utilities|Array|SetArrayElem (Variables|Default|GetItems) _array_index (Variables|/Game/Inventory/Blueprints/BP_Item.BP_Item_C|GetItem _asbp_item))
                    (goto _label)))))))))
    (:CastFailed
      (bind _asbp_normal_box (Utilities|Casting|CastToBP_Normal_Box (.HitActor (Collision|BreakHitResult _outhit))))
      (bind _asbp_valueable_box (Utilities|Casting|CastToBP_Valueable_Box _asbp_normal_box)
        (:then
          (CallFunction|ValuableItemSpawn _asbp_valueable_box))
        (:CastFailed
          (CallFunction|RandomItemSpawn _asbp_normal_box))))))

(event EventBeginPlay
  (bind _outactors (Actor|GetAllActorsOfClass "/Game/Building_Meshes/BP_Floor.BP_Floor_C"))
  (Variables|Default|SetFloor _outactors)
  (bind _returnvalue (UserInterface|CreateWidget "/Game/Inventory/Widgets/WB_Inventory.WB_Inventory_C"))
  (Variables|Default|SetInventorywidget _returnvalue)
  (Utilities|Array|Resize (Variables|Default|GetItems) 8)
  (Default|LoadInventory (Variables|Default|GetInventorywidget) self))

(event EventTick
  (params (DeltaSeconds :type Float%20%28single-precision%29)))

(event Input|KeyboardEvents|DebugKeyE
  (params (Key :type Key%20Structure :default "None") (ActionValue :type Input%20Action%20Value%20Structure))
  (bind _returnvalue (Game|GetPlayerCharacter 0))
  (bind _returnvalue_2 (Transformation|GetActorLocation _returnvalue))
  (bind _returnvalue_3 (+ _returnvalue_2 "0.000000,0.000000,-50.000000"))
  (:Pressed
    (bind _outhit (Collision|SphereTraceByChannel _returnvalue_3 _returnvalue_3 2e+02 "TraceTypeQuery1" false (Variables|Default|GetFloor) "None"))
    (bind _asbp_item (Utilities|Casting|CastToBP_Item (.HitActor (Collision|BreakHitResult _outhit)))
      (:then
        (if (Utilities|Enum|Equal(Enum) (.Name (Utilities|Struct|BreakS_ItemStruct (Variables|/Game/Inventory/Blueprints/BP_Item.BP_Item_C|GetItem _asbp_item))) (Variables|Default|GetAmmo))
          (bind _asbp_crosshair_character (Utilities|Casting|CastToBP_CrosshairCharacter (Game|Player|GetPlayerPawn 0)))
          (bind _asbp_weap_gun (Utilities|Casting|CastToBP_Weap_Gun (Variables|/Game/CT_Components/Demos/Demo_CrosshairSystem/ThirdPerson/BP_CrosshairCharacter.BP_CrosshairCharacter_C|GetWeapon _asbp_crosshair_character)))
          (Variables|/Game/CT_Components/Demos/Demo_CrosshairSystem/ThirdPerson/Weaps/BP_Weap_Gun.BP_Weap_Gun_C|Setmagazine _asbp_weap_gun (+ (Variables|/Game/CT_Components/Demos/Demo_CrosshairSystem/ThirdPerson/Weaps/BP_Weap_Gun.BP_Weap_Gun_C|Getmagazine _asbp_weap_gun) (.Quantity (Utilities|Struct|BreakS_ItemStruct (Variables|/Game/Inventory/Blueprints/BP_Item.BP_Item_C|GetItem _asbp_item)))))
          (Actor|DestroyActor _asbp_item)
          (else
            (for (_array_element _array_index) (Variables|Default|GetItems)
              (Utilities|IsValid _asbp_item
                (:Is%20Valid
                  (if (Math|Boolean|ANDBoolean (Utilities|Enum|Equal(Enum) (.Name (Utilities|Struct|BreakS_ItemStruct _array_element)) (.Name (Utilities|Struct|BreakS_ItemStruct (Variables|/Game/Inventory/Blueprints/BP_Item.BP_Item_C|GetItem _asbp_item)))) (.Stackable (Utilities|Struct|BreakS_ItemStruct (Variables|/Game/Inventory/Blueprints/BP_Item.BP_Item_C|GetItem _asbp_item))) (<= (+ (.Quantity (Utilities|Struct|BreakS_ItemStruct _array_element)) (.Quantity (Utilities|Struct|BreakS_ItemStruct (Variables|/Game/Inventory/Blueprints/BP_Item.BP_Item_C|GetItem _asbp_item)))) 5))
                    (Utilities|Array|SetArrayElem (Variables|Default|GetItems) _array_index (Utilities|Struct|MakeS_ItemStruct (.name (Variables|/Game/Inventory/Blueprints/BP_Item.BP_Item_C|GetItem _asbp_item)) (.stackable (Variables|/Game/Inventory/Blueprints/BP_Item.BP_Item_C|GetItem _asbp_item)) (+ (.Quantity (Utilities|Struct|BreakS_ItemStruct _array_element)) (.Quantity (Utilities|Struct|BreakS_ItemStruct (Variables|/Game/Inventory/Blueprints/BP_Item.BP_Item_C|GetItem _asbp_item)))) (.mesh (Variables|/Game/Inventory/Blueprints/BP_Item.BP_Item_C|GetItem _asbp_item)) (.thumnail (Variables|/Game/Inventory/Blueprints/BP_Item.BP_Item_C|GetItem _asbp_item))))
                    (Default|LoadInventory (Variables|Default|GetInventorywidget) self :!label _label)
                    (if (Utilities|Enum|Equal(Enum) (.Name (Utilities|Struct|BreakS_ItemStruct (Variables|/Game/Inventory/Blueprints/BP_Item.BP_Item_C|GetItem _asbp_item))) (Variables|Default|GetShoes))
                      (CallFunction|ShoesGetSpeedChange)
                      (elif (Utilities|Enum|Equal(Enum) (.Name (Utilities|Struct|BreakS_ItemStruct (Variables|/Game/Inventory/Blueprints/BP_Item.BP_Item_C|GetItem _asbp_item))) (Variables|Default|GetFlashLight))
                        (CallFunction|FlashlightGet)
                        (elif (Utilities|Enum|Equal(Enum) (.Name (Utilities|Struct|BreakS_ItemStruct (Variables|/Game/Inventory/Blueprints/BP_Item.BP_Item_C|GetItem _asbp_item))) (Variables|Default|GetVest))
                          (CallFunction|VestGet))))
                    (Actor|DestroyActor _asbp_item)
                    (elif (== (.Quantity (Utilities|Struct|BreakS_ItemStruct _array_element)) 0)
                      (Utilities|Array|SetArrayElem (Variables|Default|GetItems) _array_index (Variables|/Game/Inventory/Blueprints/BP_Item.BP_Item_C|GetItem _asbp_item))
                      (goto _label)))))))))
      (:CastFailed
        (bind _asbp_normal_box (Utilities|Casting|CastToBP_Normal_Box (.HitActor (Collision|BreakHitResult _outhit))))
        (bind _asbp_valueable_box (Utilities|Casting|CastToBP_Valueable_Box _asbp_normal_box)
          (:then
            (CallFunction|ValuableItemSpawn _asbp_valueable_box))
          (:CastFailed
            (CallFunction|RandomItemSpawn _asbp_normal_box)))))))

(event Input|KeyboardEvents|DebugKeyI
  (params (Key :type Key%20Structure :default "None") (ActionValue :type Input%20Action%20Value%20Structure))
  (bind _returnvalue (Game|GetPlayerController 0))
  (bind _inventorywidget (Variables|Default|GetInventorywidget))
  (:Pressed
    (if (Widget|IsVisible (Variables|Default|GetInventorywidget))
      (Widget|RemovefromParent _inventorywidget)
      (Variables|/Script/Engine.PlayerController|SetbShowMouseCursor _returnvalue false)
      (Input|SetInputModeGameOnly _returnvalue false)
      (else
        (Variables|/Script/Engine.PlayerController|SetbShowMouseCursor _returnvalue true)
        (Input|SetInputModeGameandUI _returnvalue 0 "DoNotLock" true false)
        (UserInterface|Viewport|AddtoViewport _inventorywidget 0)))))

(fn ShoesGetSpeedChange
  (bind _asbp_crosshair_character (Utilities|Casting|CastToBP_CrosshairCharacter (Game|GetPlayerCharacter 0)))
  (Variables|/Game/CT_Components/Demos/Demo_CrosshairSystem/ThirdPerson/BP_CrosshairCharacter.BP_CrosshairCharacter_C|SetShoes_having _asbp_crosshair_character true)
  (if (Game|Player|IsInputKeyDown (Game|GetPlayerController 0) "RightMouseButton")
    (Default|SetMaxWalkSpeed _asbp_crosshair_character 2.5e+02)
    (else
      (Default|SetMaxWalkSpeed _asbp_crosshair_character 6e+02))))

(fn FlashlightGet
  (bind _asbp_crosshair_character (Utilities|Casting|CastToBP_CrosshairCharacter (Game|GetPlayerCharacter 0)))
  (Variables|/Game/CT_Components/Demos/Demo_CrosshairSystem/ThirdPerson/BP_CrosshairCharacter.BP_CrosshairCharacter_C|SetFlashlight_having _asbp_crosshair_character true)
  (Variables|/Game/CT_Components/Demos/Demo_CrosshairSystem/ThirdPerson/BP_CrosshairCharacter.BP_CrosshairCharacter_C|SetFlashlight_On _asbp_crosshair_character false))

(fn VestGet
  (bind _asbp_crosshair_character (Utilities|Casting|CastToBP_CrosshairCharacter (Game|GetPlayerCharacter 0)))
  (Variables|/Game/CT_Components/Demos/Demo_CrosshairSystem/ThirdPerson/BP_CrosshairCharacter.BP_CrosshairCharacter_C|SetVest_having _asbp_crosshair_character true))

(fn RandomItemSpawn
  (params (Box_location :type Actor%20Object%20Reference))
  (bind _returnvalue (Math|Random|RandomIntegerinRange 1 24))
  (bind _spawn_ammo (Variables|Default|GetSpawn%20Ammo))
  (if (<= _returnvalue 5)
    (Variables|Default|SetSpawn_item (Variables|Default|GetSpawn%20canbeaf))
    (Game|SpawnActorfromClass "/Game/Inventory/Blueprints/BP_Item.BP_Item_C" (Transformation|GetActorTransform Box_location) "Undefined" "MultiplyWithRoot" 0 (Variables|Default|GetSpawn_item) 0 :!label _label)
    (Actor|DestroyActor Box_location)
    (elif (<= _returnvalue 10)
      (Variables|Default|SetSpawn_item (Variables|Default|GetSpawn%20Soda))
      (goto _label)
      (elif (<= _returnvalue 15)
        (Variables|Default|SetSpawn_item _spawn_ammo)
        (goto _label)
        (elif (<= _returnvalue 18)
          (Variables|Default|SetSpawn_item _spawn_ammo)
          (goto _label)
          (elif (<= _returnvalue 20)
            (Variables|Default|SetSpawn_item (Variables|Default|GetSpawn%20Vest))
            (goto _label)
            (elif (<= _returnvalue 22)
              (Variables|Default|SetSpawn_item (Variables|Default|GetSpawn%20Shoes))
              (goto _label)
              (else
                (Variables|Default|SetSpawn_item (Variables|Default|GetSpawn%20Flash))))))))))

(fn ValuableItemSpawn
  (params (Box :type Actor%20Object%20Reference))
  (bind _returnvalue (Math|Random|RandomIntegerinRange 1 18))
  (if (<= _returnvalue 5)
    (Variables|Default|SetSpawn_item (Variables|Default|GetSpawn%20Vest))
    (elif (<= _returnvalue 10)
      (Variables|Default|SetSpawn_item (Variables|Default|GetSpawn%20Shoes))
      (elif (<= _returnvalue 15)
        (Variables|Default|SetSpawn_item (Variables|Default|GetSpawn%20Flash))
        (else
          (Variables|Default|SetSpawn_item (Variables|Default|GetSpawn%20Ammo))))))
  (Game|SpawnActorfromClass "/Game/Inventory/Blueprints/BP_Item.BP_Item_C" (Transformation|GetActorTransform Box) "Undefined" "MultiplyWithRoot" 0 (Variables|Default|GetSpawn_item) 0)
  (Actor|DestroyActor Box))