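; BP_109room is a trigger Blueprint that shows the WB_109room widget when a BP_CrosshairCharacter steps onto its Event_pedal component.
; If SaveCount exceeds a threshold, it also shows the mouse cursor and pauses the game.
; Otherwise the widget displays during play, and end overlap removes only the instance created on that unpaused branch.
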(event `self.event_pedal.OnComponentBeginOverlap`
  (params (OverlappedComponent :type "PrimitiveComponent Object Reference") (OtherActor :type "Actor Object Reference") (OtherComp :type "PrimitiveComponent Object Reference") (OtherBodyIndex :type Integer) (bFromSweep :type Boolean) (SweepResult :type "HitResult Structure (by ref)"))
  (bind _returnvalue (`GameplayStatics.GetPlayerController` 0))
  (cast `/Game/CT_Components/Demos/Demo_CrosshairSystem/ThirdPerson/BP_CrosshairCharacter` OtherActor)
  (if (> (`self.SaveCount`) 2)
    (set `PlayerController.bShowMouseCursor` true _returnvalue)
    (bind _returnvalue_2 (`|CreateWidget` "/Game/UI_Asset/WB_109room.WB_109room_C" _returnvalue))
    (`UserWidget.AddToViewport` _returnvalue_2 0)
    (`GameplayStatics.SetGamePaused` true)
    (else
      (bind _returnvalue_3 (`|CreateWidget` "/Game/UI_Asset/WB_109room.WB_109room_C" (`GameplayStatics.GetPlayerController` 0)))
      (`UserWidget.AddToViewport` _returnvalue_3 0))))

(event `self.event_pedal.OnComponentEndOverlap`
  (params (OverlappedComponent :type "PrimitiveComponent Object Reference") (OtherActor :type "Actor Object Reference") (OtherComp :type "PrimitiveComponent Object Reference") (OtherBodyIndex :type Integer))
  (cast `/Game/CT_Components/Demos/Demo_CrosshairSystem/ThirdPerson/BP_CrosshairCharacter` OtherActor)
  (`Widget.RemoveFromParent` (stale `self.event_pedal.OnComponentBeginOverlap` _returnvalue_3)))

(fn `UserConstructionScript`
  (`parent.UserConstructionScript`))